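; Destructible statue actor that swaps its static mesh for a Chaos Geometry Collection when hit hard or damaged.
; A strong hit impulse breaks it once, applying external strain and a radial impulse to the collection and making it unwalkable.
; Damage above a threshold only performs the mesh swap, without setting the broken flag or applying strain.
; Chaos break events clear each broken piece's collision profile and disable the static mesh's collision.
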(event OnChaosBreakEvent(GC_Statue)
  (params (BreakEvent :type Chaos%20Break%20Event%20Structure%20%28by%20ref%29))
  ;[0.15 0.15 0.15 0.5] Chaos break event
  (Class|GeometryCollectionComponent|SetPerParticleCollisionProfileName (Variables|Default|GetGC_Statue) (Utilities|Array|MakeArray (.index BreakEvent)) "")
  (Collision|SetCollisionEnabled (Variables|Default|GetSM_Statue) "NoCollision"))

(event Custom|CE_TakeDamage
  (params (DamagedActor :type Actor%20Object%20Reference) (Damage :type Float%20%28single-precision%29) (DamageType :type Damage%20Type%20Object%20Reference) (InstigatedBy :type Controller%20Object%20Reference) (DamageCauser :type Actor%20Object%20Reference))
  ;[0.15 0.15 0.15 0.5] BeginPlay
  (if (> Damage 3e+01)
    (Rendering|SetVisibility (Variables|Default|GetSM_Statue) false false)
    (Physics|SetSimulatePhysics (Variables|Default|GetSM_Statue) false)
    (Class|GeometryCollectionComponent|SetRestCollection (Variables|Default|GetGC_Statue) "/Game/StarterContent/Props/SM_Statue_SM_Statue/GC_SM_Statue1.GC_SM_Statue1" true)))

(event EventBeginPlay
  ;[0.15 0.15 0.15 0.5] BeginPlay
  (EventDispatchers|AssignOnTakeAnyDamage (delegate Custom|CE_TakeDamage)))

(event Collision|EventHit
  (params (MyComp :type Primitive%20Component%20Object%20Reference) (Other :type Actor%20Object%20Reference) (OtherComp :type Primitive%20Component%20Object%20Reference) (bSelfMoved :type Boolean) (HitLocation :type Vector :default "0, 0, 0") (HitNormal :type Vector :default "0, 0, 0") (NormalImpulse :type Vector :default "0, 0, 0") (Hit :type Hit%20Result%20Structure%20%28by%20ref%29))
  ;[0.15 0.15 0.15 0.5] OnHit
  (if (not (Variables|Default|GetIsBroken))
    (if (> (Math|Vector|VectorLength NormalImpulse) 3e+02)
      (Variables|Default|SetIsBroken true)
      (Rendering|SetVisibility (Variables|Default|GetSM_Statue) false false)
      (Physics|SetSimulatePhysics (Variables|Default|GetSM_Statue) false)
      (Class|GeometryCollectionComponent|SetRestCollection (Variables|Default|GetGC_Statue) "/Game/StarterContent/Props/SM_Statue_SM_Statue/GC_SM_Statue1.GC_SM_Statue1" true)
      (Class|GeometryCollectionComponent|ApplyExternalStrain (Variables|Default|GetGC_Statue) 0 HitLocation 1e+02 1 1.0 5e+06)
      (Physics|AddRadialImpulse (Variables|Default|GetGC_Statue) (Transformation|GetActorLocation) 1e+02 2e+02 "RIF_Constant" false)
      (Class|PrimitiveComponent|SetWalkableSlopeOverride (Variables|Default|GetGC_Statue) (Utilities|Struct|MakeWalkableSlopeOverride "WalkableSlope_Unwalkable" 0.0)))))

(fn ConstructionScript)